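; BP_InteractableFileCabinet is a searchable file cabinet that gives its loot to the interacting player once.
; Its Interactable component, given the front prompt widget in construction, fires OnInteracted, which casts to BP_PlayerCharacter and checks HasBeenSearched.
; Each item in the ULoot component's SelectedLoot is added to inventory with a HUD loot notification, passed the whole array each time.
; Empty loot still triggers the notifier, and either outcome marks the cabinet searched.
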(event `self.Interactable.OnInteracted`
  (params (InteractingPlayer :type "Actor Object Reference"))
  (bind _selectedloot (`ULootComponent.SelectedLoot` (`self.ULoot`)))
  (bind _selectedloot_2 (`ULootComponent.SelectedLoot` (`self.ULoot`)))
  (bind _asbp_player_character (cast `/Game/Player/BP_PlayerCharacter` InteractingPlayer))
  (set `self.As BP Player Character` _asbp_player_character)
  (if (not (`self.HasBeenSearched`))
    (if (`KismetArrayLibrary.Array_IsNotEmpty` _selectedloot)
      (for _array_element _selectedloot_2
        (`/Game/UI/WBP_HUD.SetLootNotifier` (`/Game/Player/BP_PlayerCharacter.HUD` (`self.As BP Player Character`)) _selectedloot_2 1)
        (`PlayerCharacter.AddItemToInventory` (`self.As BP Player Character`) _array_element 1))
      (else
        (`/Game/UI/WBP_HUD.SetLootNotifier` (`/Game/Player/BP_PlayerCharacter.HUD` (`self.As BP Player Character`)) _selectedloot 1)))
    (set `self.HasBeenSearched` true)))

(fn `UserConstructionScript`
  (set `InteractableComponent.FrontPromptWidget` (`self.FrontPromptWidget`) (`self.Interactable`)))