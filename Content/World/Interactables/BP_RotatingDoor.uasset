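; BP_RotatingDoor is an interactable door that opens on interaction and closes itself again after a short fixed delay.
; The Interactable component's interaction event plays the Door animation forward, then replays it at a negative rate to reverse it.
; The construction script hands front and rear prompt widgets to the Interactable component.
; An unconnected leftover branch plays a sliding-door animation behind an IsOpen check and never runs.
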(event `self.ReceiveBeginPlay`)

(event `self.Interactable.OnInteracted`
  (bind _door (`self.Door`))
  (bind _door_2 (`self.Door`))
  (`SkeletalMeshComponent.SetPlayRate` _door_2 1.0)
  (`SkeletalMeshComponent.Play` _door_2 false)
  (`KismetSystemLibrary.Delay` 2.0)
  (`SkeletalMeshComponent.SetPlayRate` _door -1.0)
  (`SkeletalMeshComponent.Play` _door false))

(fn `UserConstructionScript`
  (set `InteractableComponent.FrontPromptWidget` (`self.FrontPromptWidget`) (`self.Interactable`))
  (set `InteractableComponent.RearPromptWidget` (`self.RearPromptWidget`) (`self.Interactable`)))