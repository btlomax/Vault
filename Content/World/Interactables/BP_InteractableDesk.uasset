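; Searchable desk interactable that gives its loot to the player the first time it is searched.
; Loot is generated through ULoot on BeginPlay.
; On interaction, each PossibleLoot entry is added to the player character's inventory as a single item, refreshing the door keys HUD, and HasBeenSearched blocks repeat searches.
; The construction script hands front and rear prompt widgets to the Interactable component.
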(event `self.ReceiveBeginPlay`
  (`ULootComponent.GenerateLoot` (`self.ULoot`)))

(event `self.Interactable.OnInteracted`
  (params (InteractingPlayer :type "Actor Object Reference"))
  (bind _as_bp_player_character (`self.As BP Player Character`))
  (bind _asbp_player_character (cast `/Game/Player/BP_PlayerCharacter` InteractingPlayer))
  (set `self.As BP Player Character` _asbp_player_character)
  (if (not (`self.HasBeenSearched`))
    (for _array_element (`ULootComponent.PossibleLoot` (`self.ULoot`))
      (`PlayerCharacter.AddItemToInventory` _as_bp_player_character (break `LootItem` _array_element) 1)
      (`/Game/Player/BP_PlayerCharacter.UpdateDoorKeysHUD` _as_bp_player_character))
    (set `self.HasBeenSearched` true)))

(fn `UserConstructionScript`
  (bind _interactable (`self.Interactable`))
  (set `InteractableComponent.FrontPromptWidget` (`self.FrontPromptWidget`) _interactable)
  (set `InteractableComponent.RearPromptWidget` (`self.RearPromptWidget`) _interactable))