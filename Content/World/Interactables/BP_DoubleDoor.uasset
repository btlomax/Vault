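; Interactable double door that can start locked and costs one of the player's door keys to unlock.
; An interaction on a locked door only unlocks it and updates the lock-state widget text.
; Once unlocked, interacting plays the Door animation forward, then replays it in reverse after a short delay to close it.
; The construction script hands the front, rear and lock-state widgets to the Interactable component.
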(event `self.ReceiveBeginPlay`
  (bind _aswbp_door_lock_state (cast `/Game/UI/WBP_DoorLockState` (`WidgetComponent.GetUserWidgetObject` (`self.DoorLockStateWidget`))))
  (set `self.As WBP Door Lock State` _aswbp_door_lock_state)
  (if (`self.IsLocked`)
    (`/Game/UI/WBP_DoorLockState.SetDoorLockText` (`self.As WBP Door Lock State`) "Locked")
    (else
      (`/Game/UI/WBP_DoorLockState.SetDoorLockText` (`self.As WBP Door Lock State`) "Unlocked"))))

(event `self.Interactable.OnInteracted`
  (params (InteractingPlayer :type "Actor Object Reference"))
  (bind _door (`self.Door`))
  (bind _door_2 (`self.Door`))
  (bind _as_bp_player_character (`self.As BP Player Character`))
  (bind _asbp_player_character (cast `/Game/Player/BP_PlayerCharacter` InteractingPlayer))
  (set `self.As BP Player Character` _asbp_player_character)
  (if (`self.IsLocked`)
    (if (> (`PlayerCharacter.DoorKeys` (`self.As BP Player Character`)) 0)
      (bind _result (`/Engine/EditorBlueprintResources/StandardMacros.DecrementInt` (`PlayerCharacter.DoorKeys` _as_bp_player_character))
        (:`  `
          (set `PlayerCharacter.DoorKeys` _result _as_bp_player_character)
          (set `self.IsLocked` false)
          (`/Game/UI/WBP_DoorLockState.SetDoorLockText` (`self.As WBP Door Lock State`) "Unlocked"))))
    (else
      (`SkeletalMeshComponent.SetPlayRate` _door_2 1.0)
      (`SkeletalMeshComponent.Play` _door_2 false)
      (`KismetSystemLibrary.Delay` 2.0)
      (`SkeletalMeshComponent.SetPlayRate` _door -1.0)
      (`SkeletalMeshComponent.Play` _door false))))

(fn `UserConstructionScript`
  (bind _interactable (`self.Interactable`))
  (set `InteractableComponent.FrontPromptWidget` (`self.FrontPromptWidget`) _interactable)
  (set `InteractableComponent.RearPromptWidget` (`self.RearPromptWidget`) _interactable)
  (set `InteractableComponent.DoorLockStateWidget` (`self.DoorLockStateWidget`) _interactable))