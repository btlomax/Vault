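; Interactable single door that starts locked or unlocked per IsLocked and is unlocked with a Blue Door Key from the player's inventory.
; An Interactable component receives the prompt and lock-state widgets at construction and fires OnInteracted.
; Unlocking consumes the key and updates the lock label and HUD notifier; a missing key only shows a notice.
; Later interactions play the door animation forward, then reverse it after a short delay to close automatically.
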(event `self.ReceiveBeginPlay`
  (bind _aswbp_door_lock_state (cast `/Game/UI/WBP_DoorLockState` (`WidgetComponent.GetUserWidgetObject` (`self.DoorLockStateWidget`))))
  (set `self.As WBP Door Lock State` _aswbp_door_lock_state)
  (if (`self.IsLocked`)
    (`/Game/UI/WBP_DoorLockState.SetDoorLockText` (`self.As WBP Door Lock State`) "Locked")
    (else
      (`/Game/UI/WBP_DoorLockState.SetDoorLockText` (`self.As WBP Door Lock State`) "Unlocked"))))

(event `self.Interactable.OnInteracted`
  (params (InteractingPlayer :type "Actor Object Reference"))
  (bind _singledoor (`self.SingleDoor`))
  (bind _singledoor_2 (`self.SingleDoor`))
  (bind _asbp_player_character (cast `/Game/Player/BP_PlayerCharacter` InteractingPlayer))
  (set `self.As BP Player Character` _asbp_player_character)
  (if (`self.IsLocked`)
    (if (`PlayerCharacter.HasItemInInventory` (`self.As BP Player Character`) "Blue Door Key" 1)
      (`PlayerCharacter.RemoveItemFromInventory` (`self.As BP Player Character`) "Blue Door Key" 1)
      (set `self.IsLocked` false)
      (`/Game/UI/WBP_DoorLockState.SetDoorLockText` (`self.As WBP Door Lock State`) "Unlocked")
      (`/Game/UI/WBP_HUD.SetGenericNotifier` (`/Game/Player/BP_PlayerCharacter.HUD` (`self.As BP Player Character`)) "Door unlocked!")
      (else
        (`/Game/UI/WBP_HUD.SetGenericNotifier` (`/Game/Player/BP_PlayerCharacter.HUD` (`self.As BP Player Character`)) "Need key!")))
    (else
      (`SkeletalMeshComponent.SetPlayRate` _singledoor_2 1.0)
      (`SkeletalMeshComponent.Play` _singledoor_2 false)
      (`KismetSystemLibrary.Delay` 2.0)
      (`SkeletalMeshComponent.SetPlayRate` _singledoor -1.0)
      (`SkeletalMeshComponent.Play` _singledoor false))))

(fn `UserConstructionScript`
  (set `InteractableComponent.FrontPromptWidget` (`self.FrontPromptWidget`) (`self.Interactable`))
  (set `InteractableComponent.RearPromptWidget` (`self.RearPromptWidget`) (`self.Interactable`))
  (set `InteractableComponent.DoorLockStateWidget` (`self.DoorLockStateWidget`) (`self.Interactable`)))