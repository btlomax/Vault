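; BP_InteractableDesk2 is a searchable desk that gives the player randomly or procedurally generated loot once.
; The ULoot component generates loot on BeginPlay, and the Interactable component, given front and rear prompt widgets at construction, triggers the search.
; The first player interaction adds each selected item to the inventory with a HUD notifier, or shows "Empty...".
; It then flags the desk as searched and refreshes the inventory HUD.
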(event `self.ReceiveBeginPlay`
  (`ULootComponent.GenerateLoot` (`self.ULoot`)))

(event `self.Interactable.OnInteracted`
  (params (InteractingPlayer :type "Actor Object Reference"))
  (bind _as_bp_player_character (`self.As BP Player Character`))
  (bind _selectedloot (`ULootComponent.SelectedLoot` (`self.ULoot`)))
  (bind _asbp_player_character (cast `/Game/Player/BP_PlayerCharacter` InteractingPlayer))
  (set `self.As BP Player Character` _asbp_player_character)
  (if (not (`self.HasBeenSearched_0`))
    (if (`KismetArrayLibrary.Array_IsNotEmpty` (`ULootComponent.SelectedLoot` (`self.ULoot`)))
      (for _array_element _selectedloot
        (`/Game/UI/WBP_HUD.SetLootNotifier` (`/Game/Player/BP_PlayerCharacter.HUD` _as_bp_player_character) _selectedloot 1)
        (`PlayerCharacter.AddItemToInventory` (`self.As BP Player Character`) _array_element 1))
      (else
        (`/Game/UI/WBP_HUD.SetGenericNotifier` (`/Game/Player/BP_PlayerCharacter.HUD` (`self.As BP Player Character`)) "Empty...")))
    (set `self.HasBeenSearched_0` true)
    (`/Game/UI/WBP_HUD.UpdateInventory` (`/Game/Player/BP_PlayerCharacter.HUD` _as_bp_player_character) (`PlayerCharacter.Inventory` _as_bp_player_character))))

(fn `UserConstructionScript`
  (bind _interactable (`self.Interactable`))
  (set `InteractableComponent.FrontPromptWidget` (`self.FrontPromptWidget`) _interactable)
  (set `InteractableComponent.RearPromptWidget` (`self.RearPromptWidget`) _interactable))