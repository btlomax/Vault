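; BP_PlayerVan is an interactable player van that opens a planning screen.
; On BeginPlay it creates a hidden WBP_PlanningUI and passes itself as VanRef.
; Its Interactable component, given front and rear prompt widgets during construction, triggers hiding the interacting player and showing the UI.
; OnPlanningUIClosed reverses both, using the player reference from the interaction event.
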(event `self.ReceiveBeginPlay`
  (bind _returnvalue (`|CreateWidget` "/Game/UI/WBP_PlanningUI.WBP_PlanningUI_C" null null))
  (bind _output_get (set `self.UI` _returnvalue))
  (`UserWidget.AddToViewport` _output_get 0)
  (`Widget.SetVisibility` (`self.UI`) "Hidden")
  (set `/Game/UI/WBP_PlanningUI.VanRef` self (`self.UI`)))

(event `self.Interactable.OnInteracted`
  (params (InteractingPlayer :type "Actor Object Reference"))
  (`self.SetActorHiddenInGame` InteractingPlayer true)
  (`Widget.SetVisibility` (`self.UI`) "Visible"))

(event `/Game/Interfaces/BPI_PlanningUIEvents.OnPlanningUIClosed`
  (`self.SetActorHiddenInGame` (stale `self.Interactable.OnInteracted` InteractingPlayer) false)
  (`Widget.SetVisibility` (`self.UI`) "Hidden"))

(fn `UserConstructionScript`
  (set `InteractableComponent.FrontPromptWidget` (`self.FrontPromptWidget`) (`self.Interactable`))
  (set `InteractableComponent.RearPromptWidget` (`self.RearPromptWidget`) (`self.Interactable`)))