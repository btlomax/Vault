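; Player character Blueprint that creates the player's HUD, clock and phase debug widgets on BeginPlay.
; It binds to BP_TimeManager's time events, converting the current time into an hours:minutes clock display.
; When end time is reached, it waits briefly, hides the clock and switches the game mode to the Heist phase.
; A separate event refreshes the HUD's door key count from the Inventory.
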(event `self.ReceiveBeginPlay`
  (bind _returnvalue (`|CreateWidget` "/Game/Game/Test/WBP_PhaseDebug.WBP_PhaseDebug_C"))
  (`UserWidget.AddToViewport` _returnvalue 0)
  (bind _returnvalue_2 (`|CreateWidget` "/Game/UI/WBP_Clock.WBP_Clock_C"))
  (bind _output_get (set `self.Clock` _returnvalue_2))
  (`UserWidget.AddToViewport` _output_get 0)
  (bind _outactors (`GameplayStatics.GetAllActorsOfClass` "/Game/Game/BP_TimeManager.BP_TimeManager_C"))
  (for _array_element _outactors
    _)
  (add `TimeManager.OnTimeChanged` _array_element (delegate `UpdateClock`))
  (add `TimeManager.OnEndTimeReached` _array_element (delegate `EndTimeReached`))
  (bind _returnvalue_3 (`|CreateWidget` "/Game/UI/WBP_HUD.WBP_HUD_C"))
  (bind _output_get_2 (set `self.HUD` _returnvalue_3))
  (`UserWidget.AddToViewport` _output_get_2 0)
  (`/Game/UI/WBP_HUD.SetDoorKeysText` (`self.HUD`) 0))

(event `EndTimeReached`
  (`KismetSystemLibrary.Delay` 1.0)
  (`Widget.SetVisibility` (`self.Clock`) "Hidden")
  (bind _asgm_game_mode_controller (cast `/Game/Game/GM_GameModeController` (`GameplayStatics.GetGameMode`)))
  (`GameModeController.SetGamePhase` _asgm_game_mode_controller "Heist"))

(event `UpdateClock`
  (params (CurrentTime :type "Float (single-precision)"))
  (bind _returnvalue (`KismetMathLibrary.FFloor` CurrentTime))
  (`TextBlock.SetText` (`/Game/UI/WBP_Clock.Timer` (`self.Clock`)) (`|FormatText` "{Hours}:{Minutes}" (`KismetTextLibrary.Conv_IntToText` _returnvalue false true 2) (`KismetTextLibrary.Conv_IntToText` (`KismetMathLibrary.FTrunc` (* (- CurrentTime _returnvalue) 60.0)) false true 2))))

(event `UpdateDoorKeysHUD`
  (`/Game/UI/WBP_HUD.SetDoorKeysText` (`self.HUD`) (`BlueprintMapLibrary.Map_Find` (`self.Inventory`) "DoorKey")))

(fn `UserConstructionScript`)